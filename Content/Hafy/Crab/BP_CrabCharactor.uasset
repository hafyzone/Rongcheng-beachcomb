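; Crab character Blueprint that can be picked up and dropped by a component, with no other active logic.
; Pickup releases any existing holder through Drop, records the new one in HeldBy and attaches the Mesh to it, keeping world transform.
; Drop detaches the Mesh in place and clears HeldBy, but only when the requesting component is the current holder.
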(event EventBeginPlay)

(event Collision|EventActorBeginOverlap
  (params (OtherActor :type Actor%20Object%20Reference)))

(event EventTick
  (params (DeltaSeconds :type Float%20%28single-precision%29)))

(fn ConstructionScript)

(fn Drop
  (params (ByComponent :type Scene%20Component%20Object%20Reference) (HandleIfUsed :type Physics%20Handle%20Component%20Object%20Reference))
  (if (== ByComponent (Variables|Default|GetHeldBy))
    (Transformation|DetachFromComponent (Variables|Character|GetMesh) "KeepWorld" "KeepWorld" "KeepWorld" true)
    (Variables|Default|SetHeldBy 0)
    (return false)))

(fn Pickup
  (params (ByComponent :type Scene%20Component%20Object%20Reference) (HandleIfUsed :type Physics%20Handle%20Component%20Object%20Reference))
  (if (!= (Variables|Default|GetHeldBy) 0)
    (CallFunction|Drop (Variables|Default|GetHeldBy)))
  (bind _output_get (Variables|Default|SetHeldBy ByComponent))
  (bind _returnvalue (Transformation|AttachComponentToComponent (Variables|Character|GetMesh) _output_get "None" "KeepWorld" "KeepWorld" "KeepWorld" true))
  (return _returnvalue))